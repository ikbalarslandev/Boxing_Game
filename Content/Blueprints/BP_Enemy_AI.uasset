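; BP_Enemy_AI is a melee enemy character that pursues the player and punches on reaching them.
; From BeginPlay, an AI MoveTo targets the player character; on success it plays a left punch montage, waits briefly and repeats, with no handling of failed moves.
; Hit-reaction events play montages of the opposite side: getlefthit plays the right-hit montage and getrighthit the left.
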(event Custom|get%20left%20hit
  (Animation|PlayAnimMontage "/Game/Characters/Boxer/animations/hit/right_hit_Montage.right_hit_Montage" 1.0 "None"))

(event Custom|get%20right%20hit
  (Animation|PlayAnimMontage "/Game/Characters/Boxer/animations/hit/left_hit_Montage.left_hit_Montage" 1.0 "None"))

(event Custom|Chase%20Player
  (AI|AIMoveTo self "0, 0, 0" (Game|GetPlayerCharacter 0) 1e+02 false
    (:OnSuccess
      (CallFunction|Attack)
      (Utilities|FlowControl|Delay 2.0)
      (CallFunction|ChasePlayer))))

(event Custom|Attack
  (Animation|PlayAnimMontage "/Game/Characters/Boxer/animations/punch/montages/punching_left_Montage.punching_left_Montage" 1.0 "None"))

(event Collision|EventActorBeginOverlap
  (params (OtherActor :type Actor%20Object%20Reference)))

(event EventBeginPlay
  (CallFunction|ChasePlayer))

(fn ConstructionScript)